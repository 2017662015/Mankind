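; CharacterBP is a parent character Blueprint that provides a simple state-machine skeleton for child characters.
; WatchDog compares CurrentCState with PreCState and, on a change, stores the new state and calls its handler, covering init through death.
; The OnActor handlers are empty hooks, presumably for child overrides.
; Nothing in this Blueprint calls WatchDog, and its BeginPlay, overlap and Tick events are disabled placeholders.
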(event EventBeginPlay
  (|CallParentFunction) ; 지금 이 노드는 비활성 상태입니다. \n핀을 끌어서 다른 노드를 연결하면 활성화됩니다.
)

(event Collision|EventActorBeginOverlap
  (params (OtherActor :type Actor%20Object%20Reference))
  (|CallParentFunction OtherActor) ; 지금 이 노드는 비활성 상태입니다. \n핀을 끌어서 다른 노드를 연결하면 활성화됩니다.
)

(event EventTick
  (params (DeltaSeconds :type Float%20%28single-precision%29))
  (|CallParentFunction DeltaSeconds) ; 지금 이 노드는 비활성 상태입니다. \n핀을 끌어서 다른 노드를 연결하면 활성화됩니다.
)

(fn ConstructionScript
  (|CallParentFunction))

(fn WatchDog
  (bind _currentcstate (Variables|Default|GetcurrentCState))
  ;[1 1 1] Check the state and execute the proper method
  ;;[1 1 1] Check States are different or not
  (if (Utilities|Enum|NotEqual(Enum) (Variables|Default|GetcurrentCState) (Variables|Default|GetpreCState))
    ;;[1 1 1] If currentCState is different with preCState then  copy value of currentCState to preCState
    (Variables|Default|SetpreCState _currentcstate)
    ;;[1 1 1] Execute the proper method on it's state
    (switch Utilities|FlowControl|Switch|SwitchonE_CharacterState _currentcstate
      (:NewEnumerator1
        (CallFunction|OnActorInit))
      (:NewEnumerator2
        (CallFunction|OnActorIdle))
      (:NewEnumerator3
        (CallFunction|OnActorWalk))
      (:NewEnumerator4
        (CallFunction|OnActorRun))
      (:NewEnumerator5
        (CallFunction|OnActorAttack))
      (:NewEnumerator6
        (CallFunction|OnActorDamaged))
      (:NewEnumerator7
        (CallFunction|OnActorDied)))))

(fn OnActorInit)

(fn OnActorIdle)

(fn OnActorWalk)

(fn OnActorRun)

(fn OnActorAttack)

(fn OnActorDamaged)

(fn OnActorDied)