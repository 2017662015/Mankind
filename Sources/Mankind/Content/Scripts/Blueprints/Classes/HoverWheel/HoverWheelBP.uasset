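; Rideable VR hover vehicle that the player grips with both motion controllers, then steers by hand and drives by leaning.
; Tick switches between sine bobbing when idle, settling when a player is near, rising once snapped, and moving at ride height.
; HMD offset from the axis sets throttle, while controller positions rotate the handle for yaw, even one-handed.
; Releasing both hands unsnaps, lowers the wheel to origin height, then detaches the player.
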(event EventBeginPlay
  (|CallParentFunction) ; 지금 이 노드는 비활성 상태입니다. \n핀을 끌어서 다른 노드를 연결하면 활성화됩니다.
)

(event EventTick
  (params (DeltaSeconds :type Float%20%28single-precision%29))
  (bind _axis_hoverwheel (Variables|Default|GetAxis_HoverWheel))
  (bind _updownoffset (Variables|Default|GetupDownOffset))
  (bind _downspeed (Variables|Default|GetdownSpeed))
  (|CallParentFunction DeltaSeconds)
  (if (Variables|Default|GetisSnapped)
    (if (Variables|Default|GetisRidePos)
      (CallFunction|Move)
      (else
        (HoverWheel|PlayerRideSequence _axis_hoverwheel _downspeed _updownoffset)))
    (elif (Variables|Default|GetisPlayerNear)
      (HoverWheel|PlayerNearSequence _axis_hoverwheel _downspeed :!label _label)
      (elif (Variables|Default|GetisOrigin)
        (HoverWheel|UpDownMovement _axis_hoverwheel _updownoffset)
        (else
          (goto _label))))))

(event OnComponentBeginOverlap(Collision_Handle_R)
  (params (OverlappedComponent :type Primitive%20Component%20Object%20Reference) (OtherActor :type Actor%20Object%20Reference) (OtherComp :type Primitive%20Component%20Object%20Reference) (OtherBodyIndex :type Integer) (bFromSweep :type Boolean) (SweepResult :type Hit%20Result%20Structure%20%28by%20ref%29))
  (bind _returnedscenereference (Tag|BindOverlappedRefwithTag OtherComp "ObjectNameTable" "COL_MOTCONTROL_R"))
  (if (not (Variables|Default|GetisSnapped))
    (Variables|컴포넌트|SetcolMotControllerR_reference _returnedscenereference)))

(event OnComponentBeginOverlap(Collision_Handle_L)
  (params (OverlappedComponent :type Primitive%20Component%20Object%20Reference) (OtherActor :type Actor%20Object%20Reference) (OtherComp :type Primitive%20Component%20Object%20Reference) (OtherBodyIndex :type Integer) (bFromSweep :type Boolean) (SweepResult :type Hit%20Result%20Structure%20%28by%20ref%29))
  (bind _returnedscenereference (Tag|BindOverlappedRefwithTag OtherComp "ObjectNameTable" "COL_MOTCONTROL_L"))
  (if (not (Variables|Default|GetisSnapped))
    (Variables|컴포넌트|SetcolMotControllerL_Reference _returnedscenereference)))

(event OnComponentEndOverlap(Collision_Handle_L)
  (params (OverlappedComponent :type Primitive%20Component%20Object%20Reference) (OtherActor :type Actor%20Object%20Reference) (OtherComp :type Primitive%20Component%20Object%20Reference) (OtherBodyIndex :type Integer))
  (bind (_isequal _isvaild) (Tag|CompareObjectTag OtherComp "ObjectNameTable" "COL_MOTCONTROL_L"))
  (if _isvaild
    (if _isequal
      (if (not (Variables|Default|GetisSnapped))
        (if (Utilities|IsValid (Variables|컴포넌트|GetcolMotControllerL_Reference))
          (Variables|컴포넌트|SetcolMotControllerL_Reference 0))))))

(event OnComponentEndOverlap(Collision_Handle_R)
  (params (OverlappedComponent :type Primitive%20Component%20Object%20Reference) (OtherActor :type Actor%20Object%20Reference) (OtherComp :type Primitive%20Component%20Object%20Reference) (OtherBodyIndex :type Integer))
  (bind (_isequal _isvaild) (Tag|CompareObjectTag OtherComp "ObjectNameTable" "COL_MOTCONTROL_R"))
  (if _isvaild
    (if _isequal
      (if (not (Variables|Default|GetisSnapped))
        (if (Utilities|IsValid (Variables|컴포넌트|GetcolMotControllerR_reference))
          (Variables|컴포넌트|SetcolMotControllerR_reference 0))))))

(event OnComponentBeginOverlap(Collision_CheckPlayer)
  (params (OverlappedComponent :type Primitive%20Component%20Object%20Reference) (OtherActor :type Actor%20Object%20Reference) (OtherComp :type Primitive%20Component%20Object%20Reference) (OtherBodyIndex :type Integer) (bFromSweep :type Boolean) (SweepResult :type Hit%20Result%20Structure%20%28by%20ref%29))
  (if (not (Variables|Default|GetisSnapped))
    (if (Tag|TryCompareActorbyClass OtherActor "/Game/Scripts/Blueprints/Classes/Player/PlayerBP.PlayerBP_C")
      (Variables|Default|SetisPlayerNear true))))

(event OnComponentEndOverlap(Collision_CheckPlayer)
  (params (OverlappedComponent :type Primitive%20Component%20Object%20Reference) (OtherActor :type Actor%20Object%20Reference) (OtherComp :type Primitive%20Component%20Object%20Reference) (OtherBodyIndex :type Integer))
  (if (not (Variables|Default|GetisSnapped))
    (if (Tag|TryCompareActorbyClass OtherActor "/Game/Scripts/Blueprints/Classes/Player/PlayerBP.PlayerBP_C")
      (Variables|Default|SetisPlayerNear false))))

(event EventRide
  (Callback|OnRide))

(event EventTakeOff
  (Callback|OnTakeOff))

(event EventSnapin
  (Callback|OnSnapin (Variables|컴포넌트|GetcolMotControllerR_reference) (Variables|컴포넌트|GetcolMotControllerL_Reference)))

(event EventSnapOut
  (params (motionControllerCollider_reference :type Scene%20Component%20Object%20Reference))
  (Callback|OnSnapOut motionControllerCollider_reference (Variables|컴포넌트|GetcolMotControllerL_Reference) (Variables|컴포넌트|GetcolMotControllerR_reference)))

(event EventInput
  (params (axisX :type Float%20%28single-precision%29) (axisY :type Float%20%28single-precision%29))
  ;[0 0 0] @Deprecated : was used for test, Do not bind this god damn node on live
)

(event EventMove
  (bind _currentplayer (Variables|Default|GetcurrentPlayer))
  (bind _axisy (Input|GetVerticalfromHMD 3e+01 (Variables|Default|GetAxis_HoverWheel) _currentplayer))
  (bind _axisx (Input|GetHorizontalfromController (Variables|Default|GetHoverWheel_Handle) (Variables|컴포넌트|GetcolMotControllerL_Reference) (Variables|컴포넌트|GetcolMotControllerR_reference) _currentplayer))
  (기본|ApplyMove _axisx _axisy 1e+03 1e+02 -1e+02 self))

(fn ConstructionScript
  (|CallParentFunction)
  (Callback|Init))

(fn CompareObjectTag
  (params (primitiveComponent_reference :type Primitive%20Component%20Object%20Reference) (targetStringTableNamespace :type String) (targetStringTableKey :type String))
  (bind (_outtext _returnvalue) (Class|KismetTextLibrary|FindTextinLocalizationTable targetStringTableNamespace targetStringTableKey))
  (bind _returnvalue_2 (Utilities|IsValid primitiveComponent_reference))
  (if _returnvalue_2
    (if _returnvalue
      (for _array_element (Variables|/Script/Engine.ActorComponent|GetComponentTags primitiveComponent_reference)
        (LocalVariables|Set_isEqual (Utilities|Name|Equal(Name) _array_element (Utilities|String|StringToName (Utilities|String|ToString(Text) _outtext))))))
    (return (LocalVariables|Get_isEqual) _returnvalue_2)))

(fn BindOverlappedRefwithTag
  (params (overlappedComponentReference :type Primitive%20Component%20Object%20Reference) (targetStringTableNamespace :type String) (targetStringTableTag :type String))
  (bind (_isequal _isvaild) (Tag|CompareObjectTag overlappedComponentReference targetStringTableNamespace targetStringTableTag))
  (if _isvaild
    (if _isequal
      (return overlappedComponentReference))))

(fn OnSnapin
  (params (colliderMotionController_r_reference :type Scene%20Component%20Object%20Reference) (collliderMotionController_L_reference :type Scene%20Component%20Object%20Reference))
  (bind _returnvalue (Components|GetOwner colliderMotionController_r_reference))
  (if (not (Variables|Default|GetisSnapped))
    (if (and (Utilities|IsValid colliderMotionController_r_reference) (Utilities|IsValid collliderMotionController_L_reference))
      (if (Utilities|IsValid _returnvalue)
        (Variables|Default|SetisSnapped true)
        (Variables|Default|SetcurrentPlayer _returnvalue)
        (CallFunction|Ride)))))

(fn OnRide
  (bind _currentplayer (Variables|Default|GetcurrentPlayer))
  (if (Variables|Default|GetisSnapped)
    (if (Utilities|IsValid _currentplayer)
      (Components|Activation|SetActive (Variables|Default|GetCollision_CheckPlayer) false false)
      (Transformation|AttachComponentToComponent _currentplayer (Variables|Default|GetAxis_HoverWheel) "None" "KeepWorld" "KeepWorld" "KeepWorld" true)
      (if true
        (Class|IRideable|Ride(Message) _currentplayer)))))

(fn ApplyMove
  (params (horizontalAxisValue :type Float%20%28single-precision%29) (verticalAxisValue :type Float%20%28single-precision%29) (moveSpeed :type Float%20%28single-precision%29) (maxForwardSpeed :type Float%20%28single-precision%29) (maxBackwardSpeed :type Float%20%28single-precision%29) (reference :type Actor%20Object%20Reference))
  (bind _returnvalue (Utilities|Time|GetWorldDeltaSeconds))
  (bind _returnvalue_2 (* verticalAxisValue _returnvalue moveSpeed))
  (if (Utilities|IsValid reference)
    (Transformation|AddActorWorldOffset reference (* (Math|Vector|GetForwardVector (.Rotation (Math|Transform|BreakTransform (Transformation|GetActorTransform reference)))) (Math|Float|Clamp(Float) _returnvalue_2 maxBackwardSpeed maxForwardSpeed)))
    (Class|Actor|AddActorWorldRotation (Math|Rotator|MakeRotator 0.0 0.0 horizontalAxisValue))
    (Variables|Default|SetcurrentSpeed _returnvalue_2)))

(fn OnSnapOut
  (params (motionControllerCollider_reference_input :type Scene%20Component%20Object%20Reference) (motionControllerCollider_L_reference :type Scene%20Component%20Object%20Reference) (motionControllerCollider_R_Reference :type Scene%20Component%20Object%20Reference))
  (if (Utilities|IsValid motionControllerCollider_reference_input)
    (Utilities|FlowControl|Sequence
      (:then_0
        (if (Utilities|IsValid motionControllerCollider_L_reference)
          (if (== motionControllerCollider_reference_input motionControllerCollider_L_reference)
            (Variables|컴포넌트|SetcolMotControllerL_Reference 0)
            (Development|PrintString "L Detached"))))
      (:then_1
        (if (Utilities|IsValid motionControllerCollider_R_Reference)
          (if (== motionControllerCollider_reference_input motionControllerCollider_R_Reference)
            (Variables|컴포넌트|SetcolMotControllerR_reference 0)
            (Development|PrintString "R Detached")))))))

(fn TryCompareActorbyClass
  (params (target :type Actor%20Object%20Reference) (compareTo :type Actor%20Class%20Reference))
  (if (Utilities|IsValid target)
    (return (== compareTo (Utilities|GetClass target)))))

(fn UpDownMovement
  (params (hoverWheelAxisComponent :type Scene%20Component%20Object%20Reference) (offset :type Float%20%28single-precision%29))
  (if (Utilities|IsValid hoverWheelAxisComponent)
    (Time|ElapseTime)
    (Transformation|AddWorldOffset hoverWheelAxisComponent (Math|Vector|MakeVector 0.0 0.0 (* (Utilities|Time|GetWorldDeltaSeconds) (Math|Trig|Sin(Radians) (Variables|Default|GetelapsedTime)) offset)) false false)))

(fn Init
  (Variables|Default|SetupDownOffset 1e+01)
  (Variables|Default|SetdownSpeed 1e+01))

(fn PlayerNearSequence
  (params (hoverWheelAxis_reference :type Scene%20Component%20Object%20Reference) (downSpeed :type Float%20%28single-precision%29))
  (bind _returnvalue (Transformation|GetWorldTransform hoverWheelAxis_reference))
  (bind _returnvalue_2 (Utilities|Time|GetWorldDeltaSeconds))
  (bind _originheight (Variables|Default|GetoriginHeight))
  (bind _location (Math|Transform|BreakTransform _returnvalue))
  (bind _returnvalue_3 (* _returnvalue_2 downSpeed))
  (bind (_x _y _z) (Math|Vector|BreakVector _location))
  (if (Utilities|IsValid hoverWheelAxis_reference)
    (if (== _z _originheight)
      (if (Variables|Default|GetisRidePos)
        (Variables|Default|SetisOrigin true)
        (Variables|Default|SetisRidePos false)
        (Variables|Default|SetelapsedTime 0.0)
        (CallFunction|TakeOff)
        (else
          (Variables|Default|SetisOrigin true)
          (Variables|Default|SetelapsedTime 0.0)))
      (else
        (Variables|Default|SetisOrigin false)
        (if (> _returnvalue_3 (- _z _originheight))
          (Transformation|SetWorldLocation hoverWheelAxis_reference (Math|Vector|MakeVector _x _y _originheight) false false)
          (else
            (Transformation|SetWorldLocation hoverWheelAxis_reference (Math|Vector|MakeVector _x _y (- _z _returnvalue_3)) false false)))))))

(fn OnBeginPlay
  (params (hoverWheelAxis_reference :type Scene%20Component%20Object%20Reference))
  (if (Utilities|IsValid hoverWheelAxis_reference)
    (Variables|Default|SetoriginHeight (.Z (Math|Vector|BreakVector (.Location (Math|Transform|BreakTransform (Transformation|GetWorldTransform hoverWheelAxis_reference))))))))

(fn ElapseTime
  (Variables|Default|SetelapsedTime (+ (Utilities|Time|GetWorldDeltaSeconds) (Variables|Default|GetelapsedTime))))

(fn GetVerticalfromHMD
  (params (maxOffset :type Float%20%28single-precision%29) (hoverWheelAxis_reference :type Scene%20Component%20Object%20Reference) (currentPlayerReference :type Actor%20Object%20Reference))
  (if (Utilities|IsValid hoverWheelAxis_reference)
    (if (Utilities|IsValid currentPlayerReference)
      (bind _asplayer_bp (Utilities|Casting|CastToPlayerBP currentPlayerReference))
      (return (Math|Float|Clamp(Float) (/ (.alt (Default|GetBaseandAltValuebyAngle _asplayer_bp (Math|Vector|VectorLengthXY (Default|PrependVectorXY _asplayer_bp (.Location (Math|Transform|BreakTransform (Transformation|GetWorldTransform (Variables|/Game/Scripts/Blueprints/Classes/Player/PlayerBP.PlayerBP_C|GetHMD _asplayer_bp)))) (.Location (Math|Transform|BreakTransform (Transformation|GetWorldTransform hoverWheelAxis_reference))))) (Default|GetXYAnglebyDotProduct _asplayer_bp (Math|Vector|GetForwardVector (.Rotation (Math|Transform|BreakTransform (Transformation|GetWorldTransform (Variables|/Game/Scripts/Blueprints/Classes/Player/PlayerBP.PlayerBP_C|GetHMD _asplayer_bp))))) (Math|Vector|GetRightVector (.Rotation (Math|Transform|BreakTransform (Transformation|GetWorldTransform (Variables|/Game/Scripts/Blueprints/Classes/Player/PlayerBP.PlayerBP_C|GetHMD _asplayer_bp))))) (Default|PrependVectorXY _asplayer_bp (.Location (Math|Transform|BreakTransform (Transformation|GetWorldTransform (Variables|/Game/Scripts/Blueprints/Classes/Player/PlayerBP.PlayerBP_C|GetHMD _asplayer_bp)))) (.Location (Math|Transform|BreakTransform (Transformation|GetWorldTransform hoverWheelAxis_reference))))))) maxOffset) -1.0)))))

(fn AppendRotatorValueonZ
  (params (input :type Rotator) (offset :type Float%20%28single-precision%29))
  (bind (_roll _pitch _yaw) (Math|Rotator|BreakRotator input))
  (return (Math|Rotator|MakeRotator _roll _pitch (+ _yaw offset))))

(fn GetHorizontalfromController
  (params (hoverWheelHandle_reference :type Scene%20Component%20Object%20Reference) (collider_motionController_L_reference :type Scene%20Component%20Object%20Reference) (collider_motionController_R_reference :type Scene%20Component%20Object%20Reference) (currentPlayer_reference :type Actor%20Object%20Reference))
  (bind _returnvalue (Utilities|IsValid currentPlayer_reference))
  (bind _returnvalue_2 (Transformation|GetWorldTransform collider_motionController_R_reference))
  (bind _returnvalue_3 (Transformation|GetWorldTransform collider_motionController_L_reference))
  (bind _returnvalue_4 (Transformation|GetWorldTransform hoverWheelHandle_reference))
  (bind _returnvalue_5 (Utilities|IsValid collider_motionController_L_reference))
  (bind _returnvalue_6 (Utilities|IsValid collider_motionController_R_reference))
  (bind _returnvalue_7 (Utilities|IsValid hoverWheelHandle_reference))
  (bind _location (Math|Transform|BreakTransform _returnvalue_3))
  (bind _location_2 (Math|Transform|BreakTransform _returnvalue_2))
  (bind (_location_3 _rotation) (Math|Transform|BreakTransform _returnvalue_4))
  (bind _returnvalue_8 (Math|Vector|GetForwardVector _rotation))
  (bind _returnvalue_9 (Math|Vector|GetRightVector _rotation))
  (if (Math|Boolean|ANDBoolean _returnvalue_7 _returnvalue_5 _returnvalue_6 _returnvalue)
    (bind _asplayer_bp (Utilities|Casting|CastToPlayerBP currentPlayer_reference))
    (Transformation|SetWorldRotation hoverWheelHandle_reference (Math|AppendRotatorValueonZ _rotation (Default|GetXYAnglebyDotProduct _asplayer_bp _returnvalue_8 _returnvalue_9 (Default|PrependVectorXY _asplayer_bp _location _location_2))) false false)
    (return (Math|Float|Clamp(Float) (/ (.Yaw (Math|Rotator|BreakRotator (.Rotation (Math|Transform|BreakTransform (Transformation|GetRelativeTransform hoverWheelHandle_reference))))) 45.0) -1.0))
    (elif (Math|Boolean|ANDBoolean _returnvalue_7 _returnvalue_5 _returnvalue)
      (Development|PrintString "Left Only")
      (bind _asplayer_bp_2 (Utilities|Casting|CastToPlayerBP currentPlayer_reference))
      (Transformation|SetWorldRotation hoverWheelHandle_reference (Math|AppendRotatorValueonZ _rotation (Default|GetXYAnglebyDotProduct _asplayer_bp_2 _returnvalue_8 _returnvalue_9 (Default|PrependVectorXY _asplayer_bp_2 _location _location_3))) false false)
      (return (Math|Float|Clamp(Float) (/ (.Yaw (Math|Rotator|BreakRotator (.Rotation (Math|Transform|BreakTransform (Transformation|GetRelativeTransform hoverWheelHandle_reference))))) 45.0) -1.0))
      (elif (Math|Boolean|ANDBoolean _returnvalue_7 _returnvalue_6 _returnvalue)
        (Development|PrintString "Right Only")
        (bind _asplayer_bp_3 (Utilities|Casting|CastToPlayerBP currentPlayer_reference))
        (Transformation|SetWorldRotation hoverWheelHandle_reference (Math|AppendRotatorValueonZ _rotation (Default|GetXYAnglebyDotProduct _asplayer_bp_3 _returnvalue_8 _returnvalue_9 (Default|PrependVectorXY _asplayer_bp_3 _location_3 _location_2))) false false)
        (return (Math|Float|Clamp(Float) (/ (.Yaw (Math|Rotator|BreakRotator (.Rotation (Math|Transform|BreakTransform (Transformation|GetRelativeTransform hoverWheelHandle_reference))))) 45.0) -1.0))
        (else
          (CallFunction|PreTakeOff))))))

(fn AppendRotatorValueonYZ
  (params (input :type Rotator) (offsetX :type Float%20%28single-precision%29) (offsetZ :type Float%20%28single-precision%29))
  (bind (_roll _pitch _yaw) (Math|Rotator|BreakRotator input))
  (return (Math|Rotator|MakeRotator (+ _roll offsetX) _pitch (+ _yaw offsetZ))))

(fn OnTakeOff
  (Development|PrintString "Take Off called")
  (Transformation|DetachFromActor (Variables|Default|GetcurrentPlayer) "KeepWorld" "KeepWorld" "KeepRelative")
  (bind _asplayer_bp (Utilities|Casting|CastToPlayerBP (Variables|Default|GetcurrentPlayer)))
  (Class|IRideable|TakeOff(Message) _asplayer_bp)
  (Variables|Default|SetcurrentPlayer 0))

(fn PlayerRideSequence
  (params (hoverWheelAxis_component :type Scene%20Component%20Object%20Reference) (upSpeed :type Float%20%28single-precision%29) (offset :type Float%20%28single-precision%29))
  (bind _returnvalue (Transformation|GetWorldTransform hoverWheelAxis_component))
  (bind _returnvalue_2 (Utilities|Time|GetWorldDeltaSeconds))
  (bind _originheight (Variables|Default|GetoriginHeight))
  (bind _location (Math|Transform|BreakTransform _returnvalue))
  (bind _returnvalue_3 (+ _originheight offset))
  (bind _returnvalue_4 (* _returnvalue_2 upSpeed))
  (bind (_x _y _z) (Math|Vector|BreakVector _location))
  (if (Utilities|IsValid hoverWheelAxis_component)
    (if (== _z _returnvalue_3)
      (Variables|Default|SetisRidePos true)
      (Variables|Default|SetisOrigin true)
      (Variables|Default|SetelapsedTime 0.0)
      (else
        (Variables|Default|SetisRidePos false)
        (if (> _returnvalue_4 (- _returnvalue_3 _z))
          (Transformation|SetWorldLocation hoverWheelAxis_component (Math|Vector|MakeVector _x _y _returnvalue_3) false false)
          (else
            (Transformation|SetWorldLocation hoverWheelAxis_component (Math|Vector|MakeVector _x _y (+ _z _returnvalue_4)) false false)))))))

(fn PreTakeOff
  (Variables|Default|SetisSnapped false)
  (Components|Activation|SetActive (Variables|Default|GetCollision_CheckPlayer) true false))