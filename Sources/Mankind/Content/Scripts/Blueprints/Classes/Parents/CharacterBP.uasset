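; Parent character Blueprint that provides a simple state machine over init, idle, walk, run, attack, damaged and die states.
; The construction script sets the current state to INIT and the previous to NULL, so the first check registers a change.
; Each Tick, WatchDog detects state changes, prints a debug string and fires the matching OnActor hook once, then Updatable calls that state's UpdateActor hook.
; All hooks are empty stubs.
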(event EventBeginPlay
  (|CallParentFunction) ; 지금 이 노드는 비활성 상태입니다. \n핀을 끌어서 다른 노드를 연결하면 활성화됩니다.
)

(event Collision|EventActorBeginOverlap
  (params (OtherActor :type Actor%20Object%20Reference))
  (|CallParentFunction OtherActor) ; 지금 이 노드는 비활성 상태입니다. \n핀을 끌어서 다른 노드를 연결하면 활성화됩니다.
)

(event EventTick
  (params (DeltaSeconds :type Float%20%28single-precision%29))
  (|CallParentFunction DeltaSeconds)
  (CallFunction|WatchDog)
  (CallFunction|Updatable))

(fn ConstructionScript
  (|CallParentFunction)
  (CallFunction|Init))

(fn WatchDog
  (bind _currentcstate (Variables|Default|GetcurrentCState))
  ;[1 1 1] Check the state and execute the proper method
  ;;[1 1 1] Check States are different or not
  (if (Utilities|Enum|NotEqual(Enum) (Variables|Default|GetcurrentCState) (Variables|Default|GetpreCState))
    ;;[1 1 1] State Debugger(Working on Debugging Mode)
    (CallFunction|CStateDebugger)
    ;;[1 1 1] If currentCState is different with preCState then  copy value of currentCState to preCState
    (Variables|Default|SetpreCState _currentcstate)
    ;;[1 1 1] Execute the proper method on it's state
    (switch Utilities|FlowControl|Switch|SwitchonCharacterStateEnum _currentcstate
      (:NewEnumerator1
        (CallFunction|OnActorInit))
      (:NewEnumerator2
        (CallFunction|OnActorIdle))
      (:NewEnumerator3
        (CallFunction|OnActorWalk))
      (:NewEnumerator4
        (CallFunction|OnActorRun))
      (:NewEnumerator5
        (CallFunction|OnActorAttack))
      (:NewEnumerator6
        (CallFunction|OnActorDamaged))
      (:NewEnumerator7
        (CallFunction|OnActorDie)))))

(fn OnActorInit)

(fn OnActorIdle)

(fn OnActorWalk)

(fn OnActorRun)

(fn OnActorAttack)

(fn OnActorDamaged)

(fn OnActorDie)

(fn Init
  ;[1 1 1] Change currentCState to INIT
  (Variables|Default|SetcurrentCState "NewEnumerator1")
  ;[1 1 1] Change preCState to NULL
  (Variables|Default|SetpreCState "NewEnumerator0"))

(fn CStateDebugger
  ;[1 1 1] Print States on console(Working on Debugging Mode)
  ;;[1 1 1] Print String on console
  (Development|PrintString (Utilities|String|Append (LocalVariables|GetcCStateDebugText) (Utilities|String|EnumtoString (Variables|Default|GetcurrentCState)) " " (LocalVariables|GetpCStateDebugText) (Utilities|String|EnumtoString (Variables|Default|GetpreCState))) true true "(R=0.000000,G=0.660000,B=1.000000,A=1.000000)" 5.0))

(fn UpdateActorInit)

(fn UpdateActorIdle)

(fn UpdateActorWalk)

(fn UpdateActorRun)

(fn UpdateActorAttack)

(fn UpdateActorDamaged)

(fn UpdateActorDie)

(fn Updatable
  (switch Utilities|FlowControl|Switch|SwitchonCharacterStateEnum (Variables|Default|GetcurrentCState)
    (:NewEnumerator1
      (CallFunction|UpdateActorInit))
    (:NewEnumerator2
      (CallFunction|UpdateActorIdle))
    (:NewEnumerator3
      (CallFunction|UpdateActorWalk))
    (:NewEnumerator4
      (CallFunction|UpdateActorRun))
    (:NewEnumerator5
      (CallFunction|UpdateActorAttack))
    (:NewEnumerator6
      (CallFunction|UpdateActorDamaged))
    (:NewEnumerator7
      (CallFunction|UpdateActorDie))))