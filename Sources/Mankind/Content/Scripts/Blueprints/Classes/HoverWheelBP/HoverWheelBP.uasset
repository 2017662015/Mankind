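; HoverWheelBP is a hover wheel Blueprint with left and right handle colliders and an override of a Move event, apparently meant for motion-controller grabbing.
; Handle begin-overlaps call CompareObjectTag to match the other component against side-specific motion-controller tags, but no overlap or Move logic follows yet.
; CompareObjectTag resolves tag names from a localization string table and loops over component tags, returning only the last comparison made.
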(event EventBeginPlay
  (|CallParentFunction) ; 지금 이 노드는 비활성 상태입니다. \n핀을 끌어서 다른 노드를 연결하면 활성화됩니다.
)

(event EventTick
  (params (DeltaSeconds :type Float%20%28single-precision%29))
  (|CallParentFunction DeltaSeconds) ; 지금 이 노드는 비활성 상태입니다. \n핀을 끌어서 다른 노드를 연결하면 활성화됩니다.
)

(event EventMove)

(event OnComponentBeginOverlap(Collision_Handle_R)
  (params (OverlappedComponent :type Primitive%20Component%20Object%20Reference) (OtherActor :type Actor%20Object%20Reference) (OtherComp :type Primitive%20Component%20Object%20Reference) (OtherBodyIndex :type Integer) (bFromSweep :type Boolean) (SweepResult :type Hit%20Result%20Structure%20%28by%20ref%29))
  (if (Tag|CompareObjectTag OtherComp "ObjectNameTable" "COL_MOTCONTROL_R")
    _))

(event OnComponentBeginOverlap(Collision_Handle_L)
  (params (OverlappedComponent :type Primitive%20Component%20Object%20Reference) (OtherActor :type Actor%20Object%20Reference) (OtherComp :type Primitive%20Component%20Object%20Reference) (OtherBodyIndex :type Integer) (bFromSweep :type Boolean) (SweepResult :type Hit%20Result%20Structure%20%28by%20ref%29))
  (if (Tag|CompareObjectTag OtherComp "ObjectNameTable" "COL_MOTCONTROL_L")
    _))

(event OnComponentEndOverlap(Collision_Handle_L)
  (params (OverlappedComponent :type Primitive%20Component%20Object%20Reference) (OtherActor :type Actor%20Object%20Reference) (OtherComp :type Primitive%20Component%20Object%20Reference) (OtherBodyIndex :type Integer)))

(event OnComponentEndOverlap(Collision_Handle_R)
  (params (OverlappedComponent :type Primitive%20Component%20Object%20Reference) (OtherActor :type Actor%20Object%20Reference) (OtherComp :type Primitive%20Component%20Object%20Reference) (OtherBodyIndex :type Integer)))

(fn ConstructionScript
  (|CallParentFunction))

(fn CompareObjectTag
  (params (primitiveComponent_reference :type Primitive%20Component%20Object%20Reference) (targetStringTableNamespace :type String) (targetStringTableKey :type String))
  (bind (_outtext _returnvalue) (Class|KismetTextLibrary|FindTextinLocalizationTable targetStringTableNamespace targetStringTableKey))
  (if _returnvalue
    (for _array_element (Variables|/Script/Engine.ActorComponent|GetComponentTags primitiveComponent_reference)
      (LocalVariables|Set_isEqual (Utilities|Name|Equal(Name) _array_element (Utilities|String|StringToName (Utilities|String|ToString(Text) _outtext))))))
  (return (LocalVariables|Get_isEqual)))