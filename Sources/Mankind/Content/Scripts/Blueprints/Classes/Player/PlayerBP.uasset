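; VR player Blueprint with HMD, two motion controllers and a box body collider.
; On BeginPlay it sets floor or eye tracking origin by headset type and snaps Axis onto world geometry via a downward line trace.
; Tick calls an empty Move override and SyncColliderSize, which currently only prints each controller's angle from the HMD's yaw-only forward using XY dot products.
; The collider resize code is disconnected, and its line size/center helpers are unused.
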(event EventBeginPlay
  (|CallParentFunction)
  (CallFunction|GetCurrentHMDInfo)
  (CallFunction|SetLocationtoBase))

(event Collision|EventActorBeginOverlap
  (params (OtherActor :type Actor%20Object%20Reference))
  (|CallParentFunction OtherActor) ; 지금 이 노드는 비활성 상태입니다. \n핀을 끌어서 다른 노드를 연결하면 활성화됩니다.
)

(event EventTick
  (params (DeltaSeconds :type Float%20%28single-precision%29))
  (|CallParentFunction DeltaSeconds)
  (CallFunction|Move)
  (CallFunction|SyncColliderSize 3e+01 3e+01))

(event EventInit
  ;[1 1 1 1 14] Call Init method from parent
  (|CallParentFunction)
  (Variables|Default|SetmaxRayLength 1e+04))

(event EventMove)

(event EventOnActorWalk)

(fn ConstructionScript
  (|CallParentFunction)
  (CallFunction|Init))

(fn SyncColliderSize
  (params (minColliderSize_X :type Float%20%28single-precision%29) (minColliderSize_Y :type Float%20%28single-precision%29))
  (bind _hmd (Variables|Default|GetHMD))
  (bind _returnvalue (Transformation|GetRelativeTransform _hmd))
  (bind (_location _rotation) (Math|Transform|BreakTransform _returnvalue))
  (bind _output (CallFunction|SplitandMakeRotatorwithZ _rotation))
  (bind _returnvalue_2 (Math|Vector|GetForwardVector _output))
  (Development|PrintString (Utilities|String|Append "Left Angle : " (Utilities|String|ToString(Float) (CallFunction|GetXYAnglebyDotProduct _returnvalue_2 (CallFunction|PrependVectorXY (.Location (Math|Transform|BreakTransform (Transformation|GetRelativeTransform (Variables|Default|GetMotionController_L)))) _location))) ", Right Angle" (Utilities|String|ToString(Float) (CallFunction|GetXYAnglebyDotProduct _returnvalue_2 (CallFunction|PrependVectorXY (.Location (Math|Transform|BreakTransform (Transformation|GetRelativeTransform (Variables|Default|GetMotionController_R)))) _location))))))

(fn GetCurrentHMDInfo
  (bind _output_get (Variables|Default|SetcurrentHMDDevice (Class|HeadMountedDisplayFunctionLibrary|GetHMDDeviceName)))
  (switch name _output_get
    (:Default
      (Class|HeadMountedDisplayFunctionLibrary|SetTrackingOrigin "Floor" :!label _label))
    (:OculusHMD
      (goto _label))
    (:SteamVR
      (goto _label))
    (:PSVR
      (Class|HeadMountedDisplayFunctionLibrary|SetTrackingOrigin "Eye"))))

(fn SetLocationtoBase
  (bind _axis (Variables|Default|GetAxis))
  (bind _returnvalue (Transformation|GetWorldTransform _axis))
  (bind (_location _rotation) (Math|Transform|BreakTransform _returnvalue))
  (bind (_outhit _returnvalue_2) (Collision|LineTraceForObjects _location (+ _location (* (* (Math|Vector|GetUpVector _rotation) (Variables|Default|GetmaxRayLength)) -1.0)) (Utilities|Array|MakeArray "ObjectTypeQuery2" "ObjectTypeQuery1") false 0 "None"))
  (if _returnvalue_2
    (Transformation|SetWorldLocation _axis (.ImpactPoint (Collision|BreakHitResult _outhit)) false false)))

(fn GetSignfromFloat
  (params (input :type Float%20%28single-precision%29))
  (if (== input 0.0)
    (return input)
    (else
      (return (/ input (Math|Float|Absolute(Float) input))))))

(fn GetLongLineSizewithOffset
  (params (input1 :type Float%20%28single-precision%29) (input2 :type Float%20%28single-precision%29) (offset :type Float%20%28single-precision%29))
  (bind _returnvalue (Math|Float|Absolute(Float) input1))
  (bind _returnvalue_2 (Math|Float|Absolute(Float) input2))
  (if (== (CallFunction|GetSignfromFloat input1) (CallFunction|GetSignfromFloat input2))
    (if (> _returnvalue _returnvalue_2)
      (return (+ _returnvalue offset))
      (else
        (return (+ _returnvalue_2 offset))))
    (else
      (return (+ _returnvalue _returnvalue_2 offset)))))

(fn GetCenterOfLine
  (params (input1 :type Float%20%28single-precision%29) (input2 :type Float%20%28single-precision%29))
  (bind _returnvalue (/ input2 2.0))
  (bind _returnvalue_2 (/ input1 2.0))
  (if (== (CallFunction|GetSignfromFloat input1) (CallFunction|GetSignfromFloat input2))
    (if (> (Math|Float|Absolute(Float) _returnvalue_2) (Math|Float|Absolute(Float) _returnvalue))
      (return (* _returnvalue_2 -1.0))
      (else
        (return (* _returnvalue -1.0))))
    (else
      (return (* (+ _returnvalue_2 _returnvalue) -1.0)))))

(fn GetYawAnglefromRotator
  (params (input :type Rotator))
  (return (.Yaw (Math|Rotator|BreakRotator input))))

(fn SplitandMakeRotatorwithZ
  (params (input :type Rotator))
  (return (Math|Rotator|MakeRotator 0.0 0.0 (.Yaw (Math|Rotator|BreakRotator input)))))

(fn GetXYAnglebyDotProduct
  (params (standardVectorXY :type Vector) (compareVectorXY :type Vector))
  (return (Class|KismetMathLibrary|DegAcos (/ (Math|Vector|DotProduct standardVectorXY compareVectorXY) (* (Math|Vector|VectorLengthXY standardVectorXY) (Math|Vector|VectorLengthXY compareVectorXY))))))

(fn PrependVectorXY
  (params (object :type Vector) (offset :type Vector))
  (bind (_x _y) (Math|Vector|BreakVector object))
  (bind (_x_2 _y_2) (Math|Vector|BreakVector offset))
  (return (Math|Vector|MakeVector (- _x _x_2) (- _y _y_2) 0.0)))