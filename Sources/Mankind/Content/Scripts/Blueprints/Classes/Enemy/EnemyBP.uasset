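; Enemy character that wanders walled hallways on its own and watches for the player.
; A searching/moving loop raycasts for name-matched walls and other enemies, then queues a forward step or randomly picks an open direction, reversing only at dead ends.
; Queued steps drive movement and arc turns, then snap yaw to right angles and re-center in the hallway.
; A sine-swept eye ray changes PlayerBP's state on a hit.
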(event EventBeginPlay
  (|CallParentFunction))

(event Collision|EventActorBeginOverlap
  (params (OtherActor :type Actor%20Object%20Reference))
  (|CallParentFunction OtherActor) ; 지금 이 노드는 비활성 상태입니다. \n핀을 끌어서 다른 노드를 연결하면 활성화됩니다.
)

(event EventTick
  (params (DeltaSeconds :type Float%20%28single-precision%29))
  (|CallParentFunction DeltaSeconds))

(event EventMove
  (CallFunction|MoveSequence (Variables|Default|GethallwayOffset) (Variables|Default|GetCapsuleComponent) (Utilities|String|ToString(Text) (Utilities|Text|MakeLiteralText "OBJECT_WALL")) "ForOneFrame" (Variables|Default|GetmoveSpeed))
  (CallFunction|WatchPlayer (Variables|Default|GetEyeAxis) 45.0 1e+02))

(event EventInit
  (|CallParentFunction)
  (Variables|Default|SetelapsedAngle 0.0)
  (Variables|Default|SetelapsedLength 0.0)
  (Variables|Default|SethallwayOffset 3e+02))

(event EventOnActorIdle
  ;[1 1 1] Callback Methods from WatchDog
  ;;[1 1 1] OnActorIdle Callback Method
  (Variables|Default|SetcurrentCState "NewEnumerator3"))

(event EventOnActorWalk
  ;[1 1 1] Callback Methods from WatchDog
  ;;[1 1 1] OnActorWalk Callback Method
  (Variables|Default|SetcurrentMoveSequence "NewEnumerator1"))

(event EventUpdateActorWalk
  ;[1 1 1] Callback Methods from Updatable
  ;;[1 1 1] UpdateActorWalk Callback Method
  (CallFunction|Move))

(event EventOnActorInit
  ;[1 1 1] Callback Methods from WatchDog
  ;;[1 1 1] OnActorInit Callback Method
  (Variables|Default|SetcurrentCState "NewEnumerator2"))

(fn ConstructionScript
  (|CallParentFunction))

(fn AppendRotationZAxis
  (params (angle :type Float%20%28single-precision%29) (rotator :type Rotator))
  (bind (_roll _pitch _yaw) (Math|Rotator|BreakRotator rotator))
  ;[1 1 1] Append angle on Yaw Axis of rotator and return
  (return (Math|Rotator|MakeRotator _roll _pitch (+ angle _yaw))))

(fn CompareObjectwithRay
  (params (start :type Vector) (end :type Vector) (objectTypes :type Array%20of%20EObjectTypeQuery%20Enums :default "ObjectTypeQuery1") (targetName :type String) (drawDebugType :type EDrawDebugTrace%20Enum :default "None"))
  ;[1 1 1] Raycast to destination point, compare the keyword and return boolean that equal or not and distance to the target
  ;;[1 1 1] Raycast to destination point and get the RaycastHit object
  (bind (_outhit _returnvalue) (Collision|LineTraceForObjects start end objectTypes false 0 drawDebugType true "(R=1.000000,G=0.000000,B=0.000000,A=1.000000)" "(R=0.000000,G=1.000000,B=0.000000,A=1.000000)" 3e+01))
  ;;[1 1 1] If Ray hit something, break hit result
  (if _returnvalue
    _
    (else
      _))
  (return (* (.Distance (Collision|BreakHitResult _outhit)) (Math|Conversions|ToFloat(Boolean) (Utilities|String|Contains (Utilities|GetObjectName (.HitActor (Collision|BreakHitResult _outhit))) targetName))) (Utilities|String|Contains (Utilities|GetObjectName (.HitActor (Collision|BreakHitResult _outhit))) targetName) (.HitActor (Collision|BreakHitResult _outhit))))

(fn CheckBlockedwithRay
  (params (angle :type Float%20%28single-precision%29) (length :type Float%20%28single-precision%29) (reference :type Scene%20Component%20Object%20Reference) (targetName :type String) (drawDebugType :type EDrawDebugTrace%20Enum :default "None"))
  (bind _returnvalue (Transformation|GetWorldTransform reference))
  (bind (_location _rotation) (Math|Transform|BreakTransform _returnvalue))
  ;[1 1 1] Raycast to the direction and compare the target if something hit, return the boolean that is blocked by target object or not and the distance if is blocked
  ;;[1 1 1] Run CompareObjectWithRay Method and get isEqual boolean variable and distance to the object
  (bind (_distance _isequal) (CallFunction|CompareObjectwithRay _location (+ _location (* (Math|Vector|GetForwardVector (CallFunction|AppendRotationZAxis angle _rotation)) length)) (Utilities|Array|MakeArray "ObjectTypeQuery1" "ObjectTypeQuery2") targetName drawDebugType))
  ;;[1 1 1] Return length to target and isBlocked boolean
  (return _distance _isequal))

(fn CheckSideClearwithRay
  (params (radius :type Float%20%28single-precision%29) (originAngle :type Float%20%28single-precision%29) (deltaAngle :type Integer) (sceneComponentReference :type Scene%20Component%20Object%20Reference) (targetName :type String) (drawDebugType :type EDrawDebugTrace%20Enum :default "None"))
  (bind _returnvalue (Transformation|GetWorldTransform sceneComponentReference))
  (bind (_location _rotation) (Math|Transform|BreakTransform _returnvalue))
  ;[1 1 1] Check every angle with ray until tagged object is equal with target or max delta angle
  ;;[1 1 1] Loop with delta angle
  (bind _index (Utilities|FlowControl|ForLoopwithBreak 0 deltaAngle :!label _label)
    (:LoopBody
      ;;[1 1 1] Run CompareObjectWithRay
      (bind (_distance _isequal) (CallFunction|CompareObjectwithRay _location (+ (* (Math|Vector|GetForwardVector (CallFunction|AppendRotationZAxis (- originAngle (* (CallFunction|GetPosorNegNormalized originAngle) (Math|Conversions|ToFloat(Integer) _index))) _rotation)) (/ radius (Math|Trig|Cos(Degrees) (Math|Conversions|ToFloat(Integer) _index)))) _location) (Utilities|Array|MakeArray "ObjectTypeQuery1") targetName drawDebugType))
      ;;[1 1 1] If tagged object is not equal with target, break the loop
      (if _isequal
        ;;[1 1 1] If tagged object is target, set latest angle and distance
        (LocalVariables|Set_latestAngle _index)
        (LocalVariables|Set_latestDistance _distance)
        (else
          (goto _label Break))))
    (:Completed
      ;;[1 1 1] Return is clear or not and latest distance and latest forward distance
      (return (not _isequal) (LocalVariables|Get_latestDistance) (* (LocalVariables|Get_latestDistance) (Math|Trig|Sin(Degrees) (Math|Conversions|ToFloat(Integer) (LocalVariables|Get_latestAngle))))))))

(fn GetPosorNegNormalized
  (params (input :type Float%20%28single-precision%29))
  ;[1 1 1] Calculate signed-normalized value and return
  (return (/ input (Math|Float|Absolute(Float) input))))

(fn CheckandAlignCenter
  (params (sceneComponentReference :type Scene%20Component%20Object%20Reference) (targetName :type String) (drawDebugType :type EDrawDebugTrace%20Enum :default "None"))
  (bind _returnvalue (Math|Trig|Cos(Degrees) 45.0))
  (bind __defaultmaxlength (LocalVariables|Get_defaultMaxLength))
  (Utilities|FlowControl|Sequence
    (:then_0
      (bind (_lengthtotarget _isblocked) (CallFunction|CheckBlockedwithRay -45.0 __defaultmaxlength sceneComponentReference targetName drawDebugType)))
    (:then_1
      (bind (_lengthtotarget_2 _isblocked_2) (CallFunction|CheckBlockedwithRay 45.0 __defaultmaxlength sceneComponentReference targetName drawDebugType))
      (if (and _isblocked _isblocked_2)
        (Math|Float|CompareFloat _lengthtotarget _lengthtotarget_2
          (:>
            (CallFunction|CalculateAlignRoute 45.0 (* (Math|Float|Absolute(Float) (- (* _lengthtotarget _returnvalue) (* _returnvalue _lengthtotarget_2))) (Math|Trig|Cos(Degrees) 45.0))))
          (:<
            (CallFunction|CalculateAlignRoute -45.0 (* (Math|Float|Absolute(Float) (- (* _lengthtotarget _returnvalue) (* _returnvalue _lengthtotarget_2))) (Math|Trig|Cos(Degrees) 45.0)))))
        (Variables|Default|SetisAlign true)))))

(fn CheckBothSideClear
  (params (offset :type Float%20%28single-precision%29) (sceneComponentReference :type Scene%20Component%20Object%20Reference) (targetName :type String) (drawDebugType :type EDrawDebugTrace%20Enum :default "None"))
  ;[1 1 1] Check both side clear with ray
  ;;[1 1 1] Run Reset HallwatRelCenter to get center of hallway
  (CallFunction|ResetHallwayRelCenter offset sceneComponentReference targetName drawDebugType)
  ;;[1 1 1] Run CheckSideClearWithRay to check the side is clear or not
  (Utilities|FlowControl|Sequence
    (:then_0
      (bind (_isclear _latestdistance _latestforwarddistance) (CallFunction|CheckSideClearwithRay offset -9e+01 45 sceneComponentReference targetName drawDebugType)))
    (:then_1
      (bind (_isclear_2 _latestdistance_2 _latestforwarddistance_2) (CallFunction|CheckSideClearwithRay offset 9e+01 45 sceneComponentReference targetName drawDebugType))
      ;;[1 1 1] Compare both side are clear and check latest forward has value
      (if (and (and _isclear (> _latestforwarddistance 0.0)) (and _isclear_2 (> _latestforwarddistance_2 0.0)))
        ;;[1 1 1] If both side are clear and latest forward has value, add direction forward on nextDirections array with the longest length and return the values
        (Math|Float|CompareFloat _latestforwarddistance _latestforwarddistance_2
          (:>
            (CallFunction|AddNextDirection "NewEnumerator0" 0.0 _latestforwarddistance :!label _label))
          (:==
            (goto _label))
          (:<
            (CallFunction|AddNextDirection "NewEnumerator0" 0.0 _latestforwarddistance_2 :!label _label_2)))
        (else
          ;;[1 1 1] If not, check left is clear and value isn't zero
          (if (and _isclear (> _latestforwarddistance 0.0))
            (goto _label)
            (else
              ;;[1 1 1] If not, check right is clear and value isn't zero
              (if (and _isclear_2 (> _latestforwarddistance_2 0.0))
                (goto _label_2)
                (else
                  ;;[1 1 1] If not, check left or right are clear and return the value
                  (if (or _isclear _isclear_2)
                    (return _isclear _isclear_2 offset)
                    (else
                      (return _isclear _isclear_2 _latestforwarddistance_2)))))))))
      (return _isclear _isclear_2 0.0))))

(fn CheckFrontRearClear
  (params (offset :type Float%20%28single-precision%29) (sceneComponentReference :type Scene%20Component%20Object%20Reference) (targetName :type String) (drawDebugType :type EDrawDebugTrace%20Enum :default "None"))
  (bind _returnvalue (Utilities|GetObjectName "EnemyBP"))
  (bind _returnvalue_2 (/ offset 1.0))
  ;[1 1 1] Check front and rear is clear or not with ray
  ;;[1 1 1] Run CheckBlockWithRay to each side
  (Utilities|FlowControl|Sequence
    (:then_0
      (bind _isblocked (CallFunction|CheckBlockedwithRay 0.0 _returnvalue_2 sceneComponentReference targetName drawDebugType)))
    (:then_1
      (bind _isblocked_2 (CallFunction|CheckBlockedwithRay 1.8e+02 _returnvalue_2 sceneComponentReference targetName drawDebugType)))
    (:then_2
      (bind _isblocked_3 (CallFunction|CheckBlockedwithRay 0.0 _returnvalue_2 sceneComponentReference _returnvalue drawDebugType)))
    (:then_3
      (bind _isblocked_4 (CallFunction|CheckBlockedwithRay 1.8e+02 _returnvalue_2 sceneComponentReference _returnvalue drawDebugType))
      (return (and (not _isblocked) (not _isblocked_3)) (and (not _isblocked_2) (not _isblocked_4))))))

(fn SearchDirection
  (params (offset :type Float%20%28single-precision%29) (sceneComponentReference :type Scene%20Component%20Object%20Reference) (targetName :type String) (DrawDebugType :type EDrawDebugTrace%20Enum :default "None"))
  ;[1 1 1] Search clear sides and set the next direction to move
  ;;[1 1 1] Run CheckBothSideClear method to check both sides are clear or not
  (bind (_isleftclear _isrightclear _latestdistance) (CallFunction|CheckBothSideClear offset sceneComponentReference targetName DrawDebugType))
  (if (> (Utilities|Array|Length (Variables|Default|GetnextDirections)) 0)
    _
    (else
      ;;[1 1 1] If nextDirections array is clear, Run CheckFrontRearClear to check front and rear are clear or not
      (bind (_isfrontclear _isrearclear) (CallFunction|CheckFrontRearClear offset sceneComponentReference targetName DrawDebugType))
      ;;[1 1 1] Run JudgeDirection Method to Judge Next Direction
      (CallFunction|JudgeDirection _isfrontclear _isrearclear _isleftclear _isrightclear _latestdistance)))
  ;;[1 1 1] If sequences are done, set curentMoveSequence to MOVING
  (Variables|Default|SetcurrentMoveSequence "NewEnumerator2"))

(fn JudgeDirection
  (params (isFrontClear :type Boolean) (isBackClear :type Boolean) (isLeftClear :type Boolean) (isRightClear :type Boolean) (ForwardDistance :type Float%20%28single-precision%29))
  (bind __directionarray (LocalVariables|Get_directionArray))
  (bind __directionarray_2 (LocalVariables|Get_directionArray))
  (bind _hallwayrelcenter (Variables|Default|GethallwayRelCenter))
  (bind _returnvalue (Utilities|Array|Length __directionarray))
  ;[1 1 1] Judge direction and add nextDirection struct on nextDirections array
  (Utilities|FlowControl|Sequence
    (:then_0
      ;;[1 1 1] If isFrontClear is true, Add FORWARD on _directionArray array
      (if isFrontClear
        (Utilities|Array|Add __directionarray_2 "NewEnumerator0")))
    (:then_1
      ;;[1 1 1] If isLeftClear is true, Add LEFT on _directionArray array
      (if isLeftClear
        (Utilities|Array|Add __directionarray_2 "NewEnumerator1")))
    (:then_2
      ;;[1 1 1] If isRightClear is true, Add RIGHT on _directionArray array
      (if isRightClear
        (Utilities|Array|Add __directionarray_2 "NewEnumerator2")))
    (:then_3
      ;;[1 1 1] If isBackClear is true and elses are false, Add BACKWARD setted nextDirection struct on nextDirections Array
      (if (and isBackClear (not (Math|Boolean|ORBoolean isFrontClear isRightClear isLeftClear)))
        (CallFunction|AddNextDirection "NewEnumerator3" 1.8e+02 0.0)
        (return)))
    (:then_4
      ;;[1 1 1] Execute method with the switch according to length of _directionArray array
      (switch int _returnvalue
        (:Default
          ;;[1 1 1] If length is more than 2, execute method with the switch according to randomized EnemyMoveDirEnum enum of _directionArray array
          (switch Utilities|FlowControl|Switch|SwitchonEnemyMoveDirEnum (Utilities|Array|Get(acopy) __directionarray (Math|Random|RandomInteger _returnvalue))
            (:NewEnumerator0
              ;;[1 1 1] Add nextDirection struct according to switch
              (CallFunction|AddNextDirection "NewEnumerator0" 0.0 ForwardDistance :!label _label))
            (:NewEnumerator1
              (CallFunction|AddNextDirection "NewEnumerator1" -9e+01 _hallwayrelcenter :!label _label_2))
            (:NewEnumerator2
              (CallFunction|AddNextDirection "NewEnumerator2" 9e+01 _hallwayrelcenter :!label _label_3))))
        (:0
          (CallFunction|AddNextDirection "NewEnumerator4" 0.0 0.0))
        (:1
          ;;[1 1 1] If length is 1, execute method with the switch according to EnemyMoveDirEnum enum of _directionArray array
          (switch Utilities|FlowControl|Switch|SwitchonEnemyMoveDirEnum (Utilities|Array|Get(acopy) __directionarray)
            (:NewEnumerator0
              (goto _label))
            (:NewEnumerator1
              (goto _label_2))
            (:NewEnumerator2
              (goto _label_3)))))
      (return))))

(fn MoveSequence
  (params (hallwayWidth :type Float%20%28single-precision%29) (sceneComponentReference :type Scene%20Component%20Object%20Reference) (objectName :type String) (drawDebugType :type EDrawDebugTrace%20Enum :default "None") (moveSpeed :type Float%20%28single-precision%29))
  (bind _currentmovesequence (Variables|Default|GetcurrentMoveSequence))
  ;[1 1 1] Sequence of moving - Check currentMoveSequence and Execute proper method
  ;;[1 1 1] Check currentCState is WALK or not
  (if (Utilities|Enum|Equal(Enum) (Variables|Default|GetcurrentCState) "NewEnumerator3")
    ;;[1 1 1] Check isMoving is true or not
    (if (Variables|Default|GetisMoving)
      ;;[1 1 1] If it is true, set preMoveSequence to same as currentMoveSequence and execute proper method
      (CallFunction|MovetoNextDirection moveSpeed sceneComponentReference objectName drawDebugType :!label _label)
      (else
        ;;[1 1 1] Check currentMoveSequence is different with preMoveSequence
        (if (Utilities|Enum|NotEqual(Enum) _currentmovesequence (Variables|Default|GetpreMoveSequence))
          (Variables|Default|SetpreMoveSequence _currentmovesequence)
          (switch Utilities|FlowControl|Switch|SwitchonEnemyMoveSequenceEnum _currentmovesequence
            (:NewEnumerator0
              (Variables|Default|SetcurrentCState "NewEnumerator2"))
            (:NewEnumerator1
              (CallFunction|SearchDirection hallwayWidth sceneComponentReference objectName drawDebugType))
            (:NewEnumerator2
              (goto _label))))))))

(fn AddNextDirection
  (params (nextDirection :type EnemyMoveDirEnum%20Enum :default "NewEnumerator0") (angle :type Float%20%28single-precision%29) (length :type Float%20%28single-precision%29))
  ;[1 1 1] Make NextDirectionStruct struct and add it on nextDirections array
  (Utilities|Array|Add (Variables|Default|GetnextDirections) (Utilities|Struct|MakeNextDirectionStruct nextDirection length angle)))

(fn MovetoNextDirection
  (params (moveSpeed :type Float%20%28single-precision%29) (sceneComponentReference :type Scene%20Component%20Object%20Reference) (targetName :type String) (drawDebugType :type EDrawDebugTrace%20Enum :default "None"))
  (bind _nextdirections (Variables|Default|GetnextDirections))
  (bind _output (Utilities|Array|Get(acopy) _nextdirections))
  (bind (_direction _length _angle) (Utilities|Struct|BreakNextDirectionStruct _output))
  ;[1 1 1] Check the items of nextDirection and execute the proper method as the item of nextDirection array
  ;;[1 1 1] Check isMoving variable is true or not
  (if (Variables|Default|GetisMoving)
    _
    (else
      ;;[1 1 1] If isMoving is false, set isMoving as true
      (Variables|Default|SetisMoving true)))
  ;;[1 1 1] Execute the proper method according to switch
  (switch Utilities|FlowControl|Switch|SwitchonEnemyMoveDirEnum _direction
    (:NewEnumerator0
      (if (> (Variables|Default|GetelapsedLength) _length)
        ;;[1 1 1] Remove first item of nextDirection
        (Utilities|Array|RemoveIndex _nextdirections :!label _label)
        (Variables|Default|SetelapsedLength 0.0)
        (Variables|Default|SetelapsedAngle 0.0)
        ;;[1 1 1] Check nextDirections array has another items or not
        (if (not (> (Utilities|Array|Length _nextdirections) 0))
          ;;[1 1 1] If there's no item in nextDirections array, set isMoving as false and set currentMoveSequence to SEARCHING
          (Variables|Default|SetisAlign false)
          (Variables|Default|SetisMoving false)
          (Variables|Default|SetcurrentMoveSequence "NewEnumerator1"))
        (else
          (CallFunction|MoveForward sceneComponentReference moveSpeed))))
    (:NewEnumerator1
      (if (< (Math|Float|Absolute(Float) (Variables|Default|GetelapsedAngle)) (Math|Float|Absolute(Float) _angle)) :!label _label_2
        (CallFunction|TurnasAngle sceneComponentReference moveSpeed _angle _length)
        (CallFunction|MoveForward sceneComponentReference moveSpeed)
        (else
          ;;;[1 1 1] Check isAlign is true or not, if false, Execute CheckAndAlignCenter Function
          (if (Variables|Default|GetisAlign)
            (goto _label)
            (else
              (CallFunction|CalibrateRotation sceneComponentReference)
              ;;[1 1 1] After turn left or right, run CheckAndAlignCenter Function to Align as center
              (CallFunction|CheckandAlignCenter sceneComponentReference targetName drawDebugType)
              (goto _label))))))
    (:NewEnumerator2
      (goto _label_2))
    (:NewEnumerator3
      (if (< (Math|Float|Absolute(Float) (Variables|Default|GetelapsedAngle)) (Math|Float|Absolute(Float) _angle))
        (CallFunction|TurnasAngle sceneComponentReference moveSpeed _angle _length)
        (else
          (CallFunction|CalibrateRotation sceneComponentReference)
          (goto _label))))
    (:NewEnumerator4
      (Variables|Default|SetcurrentMoveSequence "NewEnumerator0"))))

(fn MoveForward
  (params (sceneComponentReference :type Scene%20Component%20Object%20Reference) (moveSpeed :type Float%20%28single-precision%29))
  (bind _returnvalue (Utilities|Time|GetWorldDeltaSeconds))
  (bind _returnvalue_2 (* moveSpeed _returnvalue))
  ;[1 1 1] Calculate the route for moving and apply movement
  ;;[1 1 1] Update elapsedLength with new value
  (Variables|Default|SetelapsedLength (+ _returnvalue_2 (Variables|Default|GetelapsedLength)))
  ;;[1 1 1] Add the offset to world transform
  (Transformation|AddWorldOffset sceneComponentReference (* (Math|Vector|GetForwardVector (.Rotation (Math|Transform|BreakTransform (Transformation|GetWorldTransform sceneComponentReference)))) _returnvalue_2) false false))

(fn TurnasAngle
  (params (sceneComponentReference :type Scene%20Component%20Object%20Reference) (moveSpeed :type Float%20%28single-precision%29) (deltaAngle :type Float%20%28single-precision%29) (radius :type Float%20%28single-precision%29))
  (bind _returnvalue (Transformation|GetWorldTransform sceneComponentReference))
  (bind _returnvalue_2 (Utilities|Time|GetWorldDeltaSeconds))
  (bind _output (CallFunction|GetPosorNegNormalized deltaAngle))
  (bind _rotation (Math|Transform|BreakTransform _returnvalue))
  (bind _returnvalue_3 (* moveSpeed _returnvalue_2))
  (bind _returnvalue_4 (/ _returnvalue_3 radius))
  (bind _returnvalue_5 (* _returnvalue_3 _output))
  (bind _returnvalue_6 (Class|KismetMathLibrary|DegAsin _returnvalue_4))
  ;[1 1 1] Calculate the route for turning and apply turn
  ;;[1 1 1] Check radius is available or not
  (if (> radius 0.0)
    ;;[1 1 1] Update elapsedAngle with new value
    (Variables|Default|SetelapsedAngle (+ _returnvalue_6 (Variables|Default|GetelapsedAngle)))
    ;;[1 1 1] Set world rotation
    (Transformation|SetWorldRotation sceneComponentReference (CallFunction|AppendRotationZAxis (* (CallFunction|GetPosorNegNormalized deltaAngle) _returnvalue_6) _rotation) false false)
    (else
      (Variables|Default|SetelapsedAngle (+ (Variables|Default|GetelapsedAngle) _returnvalue_5))
      (Transformation|SetWorldRotation sceneComponentReference (CallFunction|AppendRotationZAxis _returnvalue_5 _rotation) false false))))

(fn ResetHallwayRelCenter
  (params (length :type Float%20%28single-precision%29) (reference :type Scene%20Component%20Object%20Reference) (targetName :type String) (drawDebugType :type EDrawDebugTrace%20Enum :default "None"))
  ;[1 1 1] Get avarage width length of hallway with CheckBlockedWithRay Method
  ;;[1 1 1] Execute CheckBlockedWithRay for check each sides are blocked or not
  (Utilities|FlowControl|Sequence
    (:then_0
      (bind (_lengthtotarget _isblocked) (CallFunction|CheckBlockedwithRay -9e+01 length reference targetName drawDebugType)))
    (:then_1
      (bind (_lengthtotarget_2 _isblocked_2) (CallFunction|CheckBlockedwithRay 9e+01 length reference targetName drawDebugType))
      ;;[1 1 1] If each sides are blocked, get average of distance and set to hallwayRelCenter
      (if (and _isblocked _isblocked_2)
        (Variables|Default|SethallwayRelCenter (/ (+ _lengthtotarget _lengthtotarget_2) 2.0))))))

(fn CalculateAlignRoute
  (params (angle :type Float%20%28single-precision%29) (offset :type Float%20%28single-precision%29))
  (bind _returnvalue (/ offset 1.0))
  (if (> angle 0.0)
    (Utilities|FlowControl|Sequence
      (:then_0
        (CallFunction|AddNextDirection "NewEnumerator1" -45.0 _returnvalue :!label _label))
      (:then_1
        (CallFunction|AddNextDirection "NewEnumerator2" 45.0 _returnvalue :!label _label_2)))
    (else
      (Utilities|FlowControl|Sequence
        (:then_0
          (goto _label_2))
        (:then_1
          (goto _label))))))

(fn CalibrateRotation
  (params (sceneComponentReference :type Scene%20Component%20Object%20Reference))
  (bind _returnvalue (Transformation|GetWorldTransform sceneComponentReference))
  (bind _rotation (Math|Transform|BreakTransform _returnvalue))
  (bind _yaw (Math|Rotator|BreakRotator _rotation))
  (bind _returnvalue_2 (Math|Float|Absolute(Float) _yaw))
  (bind _output (CallFunction|GetPosorNegNormalized _yaw))
  (bind _returnvalue_3 (Math|Float|%(Float) _returnvalue_2 9e+01))
  (bind _returnvalue_4 (* _output -1.0))
  (bind _returnvalue_5 (- 9e+01 _returnvalue_3))
  (bind _returnvalue_6 (* _returnvalue_3 _returnvalue_4))
  (bind _returnvalue_7 (* _returnvalue_5 _output))
  (bind _returnvalue_8 (Math|Rotator|MakeRotator 0.0 0.0 _returnvalue_7))
  (Development|PrintString (Utilities|String|Append "Previous : " (Utilities|String|ToString(Float) _yaw)))
  (Math|Float|CompareFloat (Math|Float|NormalizetoRange _returnvalue_3 0.0 9e+01) 0.5
    (:>
      (Development|PrintString (Utilities|String|Append "Target Angle : " (Utilities|String|ToString(Float) _returnvalue_5) (Utilities|String|ToString(Rotator) _returnvalue_8)))
      (Transformation|AddWorldRotation sceneComponentReference _returnvalue_8 false false))
    (:<
      (Development|PrintString (Utilities|String|Append "Target Angle : " (Utilities|String|ToString(Float) _returnvalue_6)))
      (Transformation|AddWorldRotation sceneComponentReference (Math|Rotator|MakeRotator 0.0 0.0 _returnvalue_6) false false)))
  (Development|PrintString (Utilities|String|Append "Now : " (Utilities|String|ToString(Float) _yaw))))

(fn WatchPlayer
  (params (eyeAxis_reference :type Scene%20Component%20Object%20Reference) (angleOffset :type Float%20%28single-precision%29) (rayLength :type Float%20%28single-precision%29))
  (bind _returnvalue (Transformation|GetWorldTransform eyeAxis_reference))
  (bind (_location _rotation) (Math|Transform|BreakTransform _returnvalue))
  (if (Utilities|IsValid eyeAxis_reference)
    (bind (_distance _isequal _returnobject) (CallFunction|CompareObjectwithRay _location (+ (* (Math|Vector|GetForwardVector (CallFunction|AppendRotationZAxis (* angleOffset (Math|Trig|Sin(Radians) (Actor|GetGameTimeSinceCreation))) _rotation)) rayLength) _location) (Utilities|Array|MakeArray "ObjectTypeQuery2") "PlayerBP" "None"))
    (if _isequal
      (bind _asplayer_bp (Utilities|Casting|CastToPlayerBP _returnobject))
      (Variables|/Game/Scripts/Blueprints/Classes/Parents/CharacterBP.CharacterBP_C|SetcurrentCState _asplayer_bp "NewEnumerator7"))))